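; Boss rocket turret that periodically launches explosive rockets on behalf of its owning BP_CharacterEnemy_Boss.
; On BeginPlay, the server starts a looping timer that checks the boss's health and plays the Shoot timeline while it is alive.
; The timeline's Shoot event spawns a BP_RocketTurret projectile just ahead of the Arrow and initializes it with hardcoded projectile info.
; The timer is cleared once the boss's health is depleted.
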(event Custom|FireRocket
  (bind _returnvalue (Components|GetOwner))
  (bind _returnvalue_2 (Math|Transform|MakeTransform "-30.000000, 0,0.000000"))
  (bind _returnvalue_3 (Math|Transform|MakeTransform "-20.000000, 0, 0" "0, 0, 0" "10.000000,10.000000,10.000000"))
  (bind _arrow (Variables|Default|GetArrow))
  (bind _projectileinfo (Utilities|Struct|MakeProjectileInfo "/Game/Blueprint/Turret/BP_RocketTurret.BP_RocketTurret_C" "/Game/Items/GameActor/Weapons/BossRocketLauncher/Rocket/Mesh/SM_Rocket.SM_Rocket" _returnvalue_3 "/Game/MilitaryWeapDark/FX/P_RocketLauncher_Trail_01.P_RocketLauncher_Trail_01" _returnvalue_2 1.0 2e+01 5e+02 1e+03 "SurfaceType_Default" 0 "SurfaceType_Default" 0 "/Game/MilitaryWeapDark/FX/P_RocketLauncher_Explosion_01.P_RocketLauncher_Explosion_01" "/Game/MilitaryWeapDark/Sound/RocketLauncher/RocketLauncher_Explosion_Cue.RocketLauncher_Explosion_Cue" 3e+02 1.5e+02 6e+01 2.0))
  (bind _asbp_character_enemy_boss (Utilities|Casting|CastToBP_CharacterEnemy_Boss _returnvalue))
  (Utilities|IsValid (Variables|/Game/Blueprint/EnemyCharacter/BP_CharacterEnemy_Base.BP_CharacterEnemy_Base_C|GetTDSHealth _asbp_character_enemy_boss)
    (:Is%20Valid
      (bind _returnvalue_4 (Class|TDSHealthComponent|GetCurrentHealth (Variables|/Game/Blueprint/EnemyCharacter/BP_CharacterEnemy_Base.BP_CharacterEnemy_Base_C|GetTDSHealth _asbp_character_enemy_boss)))
      (if (> _returnvalue_4 0.0)
        (Timeline|Shoot PlayFromStart
          (:Shoot
            (bind _returnvalue_5 (Game|SpawnActorfromClass "/Game/Blueprint/Turret/BP_RocketTurret.BP_RocketTurret_C" (Math|Transform|MakeTransform (+ (Math|Vector|GetForwardVector _arrow) (Transformation|GetWorldLocation _arrow)) (Transformation|GetWorldRotation _arrow)) "AlwaysSpawn" _returnvalue (.ProjectileInitSpeed (Utilities|Struct|BreakProjectileInfo _projectileinfo)) 0))
            (Class|ProjectileDefault|InitProjectile _returnvalue_5 _projectileinfo)))
        (else
          (Utilities|Time|ClearandInvalidateTimerbyHandle (Variables|Default|GetFireRocket_HandleTimer)))))))

(event EventBeginPlay
  (Networking|SwitchHasAuthority
    (:Authority
      (if (Networking|IsServer)
        (bind _returnvalue (Utilities|Time|SetTimerbyEvent (delegate Custom|FireRocket) 3.0 true))
        (Variables|Default|SetFireRocket_HandleTimer _returnvalue)))))

(fn ConstructionScript)