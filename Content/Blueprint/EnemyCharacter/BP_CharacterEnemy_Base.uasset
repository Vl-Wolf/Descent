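; Base enemy character with health, light and heavy melee attacks, hit reactions and ammo-style weapon-type drops on death.
; TDSHealth events spawn damage numbers and drive server-rolled confusion, flinch and temporary slowdown, gated by movement and attack flags.
; Attacks and death replicate montages via multicast; on authority, attack notifies run sphere traces damaging Player-tagged actors.
; Death unpossesses, drops the randomly pre-rolled item and ragdolls on authority after the montage.
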(event OnHealthChange(TDSHealth)
  (params (Health :type Float%20%28single-precision%29) (Damage :type Float%20%28single-precision%29))
  (bind _returnvalue (Game|SpawnActorfromClass "/Game/Widget/Damage/BP_DispalyDamageActor.BP_DispalyDamageActor_C" (Math|Transform|MakeTransform (+ (+ (Math|Vector|MakeVector (Math|Random|RandomFloatinRange 1e+01 1e+01) (Math|Random|RandomFloatinRange -1e+01 1e+01) 0.0) (Variables|Default|GetLocalPointSpawnHealthNumber)) (Transformation|GetActorLocation))) "Undefined" 0 0))
  (Default|InitActor _returnvalue Health Damage)
  (Networking|SwitchHasAuthority
    (:Authority
      (if (> (Math|Random|RandomFloat) (Variables|Chance|GetConfusionChance))
        (CallFunction|ConfusionEnabledTimer)
        (else
          (CallFunction|HitAnim)))
      (if (> (Math|Random|RandomFloat) (Variables|Chance|GetSlowDownSpeedChance))
        (Variables|Default|SetSlowDownSpeed true)
        (Utilities|Time|SetTimerbyEvent (delegate Custom|SlowDownDisableed) 2.0)))))

(event OnDead(TDSHealth)
  (bind _deathanim (Variables|Default|GetDeathAnim))
  (Networking|SwitchHasAuthority
    (:Authority
      (Variables|Default|SetSelectedDead (Utilities|Array|Get(acopy) _deathanim (- (Utilities|Array|Length _deathanim) 1)))
      (CallFunction|DeadEventMulticast (Variables|Default|GetSelectedDead)))))

(event Custom|SlowDownDisableed
  (Variables|Default|SetSlowDownSpeed false))

(event Custom|MeleeAttackLight_Multicast
  (params (SelectedLightAttack :type Anim%20Montage%20Object%20Reference))
  (bind _baselightdamage (Variables|Combat|GetBaseLightDamage))
  (Networking|SwitchHasAuthority
    (:Authority
      (bind _notifyname (Animation|Montage|PlayMontage (Variables|Character|GetMesh) SelectedLightAttack)
        (:OnCompleted
          (CallFunction|SetStateAttack true :!label _label))
        (:OnInterrupted
          (goto _label))
        (:OnNotifyBegin
          (if (Utilities|Name|Equal(Name) _notifyname "Attack")
            (Utilities|MeleeTrace 5e+01 1.5e+02 (Math|Random|RandomFloatinRange (+ _baselightdamage 2e+01) (- _baselightdamage 1e+01)) (Variables|Combat|GetLightRadius))))))
    (:Remote
      (Animation|PlayAnimMontage SelectedLightAttack 1.0 "None"))))

(event Custom|MeleeAttackHeavy_Multicast
  (params (SelectedHeavyAttack :type Anim%20Montage%20Object%20Reference))
  (bind _baseheavydamage (Variables|Combat|GetBaseHeavyDamage))
  (Networking|SwitchHasAuthority
    (:Authority
      (bind _notifyname (Animation|Montage|PlayMontage (Variables|Character|GetMesh) SelectedHeavyAttack)
        (:OnCompleted
          (CallFunction|SetStateMovement true :!label _label)
          (CallFunction|SetStateAttack true))
        (:OnInterrupted
          (goto _label))
        (:OnNotifyBegin
          (if (Utilities|Name|Equal(Name) _notifyname "Attack")
            (Utilities|MeleeTrace 5e+01 (Variables|Combat|GetEndHeavyTraceDistance) (Math|Random|RandomFloatinRange (+ _baseheavydamage 5e+01) (- _baseheavydamage 1e+01)) (Variables|Combat|GetHeavyRadius))))))
    (:Remote
      (Animation|PlayAnimMontage SelectedHeavyAttack 1.0 "None"))))

(event Custom|PlayAnim_Multicast
  (params (AnimMontage :type Anim%20Montage%20Object%20Reference) (InPlayRate :type Float%20%28single-precision%29) (StartSectionName :type Name))
  (Animation|PlayAnimMontage AnimMontage InPlayRate StartSectionName))

(event Custom|DeadEvent_Multicast
  (params (SelectedDead :type Anim%20Montage%20Object%20Reference))
  (bind _dropitemcomponent (Variables|Default|GetDropItemComponent))
  (Networking|SwitchHasAuthority
    (:Authority
      (Animation|Montage|PlayMontage (Variables|Character|GetMesh) SelectedDead
        (:then
          (Components|Movement|StopMovementImmediately (Variables|Character|GetCharacterMovement))
          (Pawn|UnPossess (Pawn|GetController))
          (Actor|SetLifeSpan 2e+01)
          (CallFunction|SetStateMovement false)
          (CallFunction|SetStateAttack false)
          (Utilities|IsValid _dropitemcomponent
            (:Is%20Valid
              (Default|Drop _dropitemcomponent))))
        (:OnCompleted
          (CallFunction|EnableRagdoll))))
    (:Remote
      (Animation|PlayAnimMontage SelectedDead 1.0 "None"))))

(event Custom|EnableRagdoll
  (bind _mesh (Variables|Character|GetMesh))
  (Collision|SetCollisionEnabled _mesh "PhysicsOnly")
  (Collision|SetCollisionResponsetoChannel (Variables|Default|GetCapsuleComponent) "ECC_Pawn" "ECR_Ignore")
  (Collision|SetCollisionProfileName _mesh "PhysicsActor" true :!class /Script/Engine.PrimitiveComponent)
  (Physics|SetSimulatePhysics _mesh true)
  (Collision|SetCollisionObjectType _mesh "ECC_PhysicsBody"))

(event EventTick
  (params (DeltaSeconds :type Float%20%28single-precision%29))
  (Variables|Default|SetDeltaTime DeltaSeconds)
  (Utilities|ChangeSpeedbyHit))

(event EventBeginPlay
  (CallFunction|InitDropComponent))

(event EventMeleeAttackHeavy
  (bind _heavyattackanim (Variables|Combat|GetHeavyAttackAnim))
  (CallFunction|SetStateAttack false)
  (CallFunction|SetStateMovement false)
  (Variables|Default|SetSelectedHeavyAttack (Utilities|Array|Get(acopy) _heavyattackanim (Math|Random|RandomInteger (Utilities|Array|Length _heavyattackanim))))
  (CallFunction|MeleeAttackHeavyMulticast (Variables|Default|GetSelectedHeavyAttack)))

(event EventMeleeAttackLight
  (bind _lightattackanim (Variables|Combat|GetLightAttackAnim))
  (CallFunction|SetStateAttack false)
  (Variables|Default|SetSelectedLightAttack (Utilities|Array|Get(acopy) _lightattackanim (Math|Random|RandomInteger (Utilities|Array|Length _lightattackanim))))
  (CallFunction|MeleeAttackLightMulticast (Variables|Default|GetSelectedLightAttack)))

(event Game|Damage|EventAnyDamage
  (params (Damage :type Float%20%28single-precision%29) (DamageType :type Damage%20Type%20Object%20Reference) (InstigatedBy :type Controller%20Object%20Reference) (DamageCauser :type Actor%20Object%20Reference))
  (Class|TDSHealthComponent|ChangeHealthValueonServer (Variables|Default|GetTDSHealth) (* Damage -1.0))
  (Variables|Default|SetLastInstigator InstigatedBy))

(fn ConstructionScript)

(fn DestroyActor
  (Actor|DestroyActor))

(fn SetStateMovement
  (params (CanMove :type Boolean))
  (Variables|Combat|SetCanMovePawn CanMove))

(fn SetStateAttack
  (params (CanAttack :type Boolean))
  (Variables|Combat|SetCanAttackPawn CanAttack))

(fn DeadEvent
  (bind _dropitemcomponent (Variables|Default|GetDropItemComponent))
  (Pawn|UnPossess (Pawn|GetController))
  (Actor|SetLifeSpan 2e+01)
  (CallFunction|SetStateMovement false)
  (CallFunction|SetStateAttack false)
  (Utilities|IsValid _dropitemcomponent
    (:Is%20Valid
      (Default|Drop _dropitemcomponent))))

(fn InitDropComponent
  (Networking|SwitchHasAuthority
    (:Authority
      (if (> (Math|Random|RandomFloat) (Variables|Chance|GetDropChance))
        (bind _returnvalue (AddComponent|AddBPDropItemComponent))
        (Variables|Default|SetDropItemComponent _returnvalue)
        (bind _output_get (Variables|/Game/Blueprint/ActorComponent/BP_DropItemComponent.BP_DropItemComponent_C|SetType _returnvalue (Utilities|Select :Index (Math|Random|RandomIntegerinRange 0 3) :Option%200 "RifleType" :Option%201 "ShotGunType" :Option%202 "SniperRifle" :Option%203 "GrenadeLauncher")))
        (Utilities|FlowControl|Sequence
          (:then_0
            (switch Utilities|FlowControl|Switch|SwitchonEWeaponType _output_get
              (:RifleType
                (LocalVariables|SetCout 30))
              (:ShotGunType
                (LocalVariables|SetCout 6))
              (:SniperRifle
                (LocalVariables|SetCout 12))
              (:GrenadeLauncher
                (LocalVariables|SetCout 2))))
          (:then_1
            (Variables|/Game/Blueprint/ActorComponent/BP_DropItemComponent.BP_DropItemComponent_C|SetCout _returnvalue (LocalVariables|GetCout))))))))

(fn ConfusionEnabledTimer
  (bind _consfusionanim (Variables|Default|GetConsfusionAnim))
  (CallFunction|SetStateMovement false)
  (bind _output_get (Variables|Default|SetCurrentMontage (Utilities|Array|Get(acopy) _consfusionanim (Math|Random|RandomIntegerinRange 0 (- (Utilities|Array|Length _consfusionanim) 1)))))
  (bind _returnvalue (Animation|GetPlayLength _output_get))
  (Utilities|Time|SetTimerbyFunctionName 0 "ConfusionDisabledTimer" _returnvalue)
  (CallFunction|PlayAnimMulticast (Variables|Default|GetCurrentMontage) 1.0 "None")
  (Variables|/Script/Engine.CharacterMovementComponent|SetMaxWalkSpeed (Variables|Character|GetCharacterMovement) 0.0)
  (Variables|Default|SetbIsConfused true))

(fn ConfusionDisabledTimer
  (CallFunction|SetStateMovement true)
  (Variables|/Script/Engine.CharacterMovementComponent|SetMaxWalkSpeed (Variables|Character|GetCharacterMovement) 4e+02))

(fn HitAnim
  (if (not (Variables|Default|GetbIsConfused))
    (if (> (Math|Random|RandomFloat) (Variables|Chance|GetHitAnimChance))
      (Animation|PlayAnimMontage "/Game/Characetrs/EnemyCharacter/Anim/Hit/Maynard_Hit_2_Montage.Maynard_Hit_2_Montage" 1.0 "None"))))

(fn CanAttack
  (return (Variables|Combat|GetCanAttackPawn)))

(fn CanMove
  (return (Variables|Combat|GetCanMovePawn)))