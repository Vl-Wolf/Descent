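; BP_Character is the networked player character with weapons, inventory, customizable body and cape colors, and an adjustable zoom camera boom.
; A looping overlap check drives the pickup prompt and holding interact picks weapons up, while drops spawn pickup actors.
; Inventory, health and weapon events update HUD widgets, multicast montages and show blood via decals and a dynamic material.
; The server emits periodic AI noise, saves inventory on unpossess and requests respawn or spectating on death.
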(event OnHealthChange(HealthComponent)
  (params (Health :type Float%20%28single-precision%29) (Damage :type Float%20%28single-precision%29))
  (bind _returnvalue (Math|Float|MapRangeClamped Health 5e+01 1e+02 1.0 0.0))
  (bind _mesh (Variables|Character|GetMesh))
  (bind _returnvalue_2 (Rendering|Material|GetMaterial _mesh 0))
  ;[1 1 1] HealthChange
  (Utilities|FlowControl|Sequence
    (:then_0
      (if (< Damage 0.0)
        (if (> (Math|Random|RandomFloat) 0.6)
          (Rendering|Decal|SpawnDecalatLocation (Utilities|Select :Index (Math|Random|RandomIntegerinRange 0 2) :Option%200 "/Game/MS_Blood/Decal/010_Blood_Stain_sgfjdepc/010_Blood_Stain_sgfjdepc_8K_inst.010_Blood_Stain_sgfjdepc_8K_inst" :Option%201 "/Game/MS_Blood/Decal/13_Blood_Stain_sheadaac/13_Blood_Stain_sheadaac_8K_inst.13_Blood_Stain_sheadaac_8K_inst" :Option%202 "/Game/MS_Blood/Decal/15_Blood_Stain_sg3bbd2c/15_Blood_Stain_sg3bbd2c_8K_inst.15_Blood_Stain_sg3bbd2c_8K_inst") "30.000000,60.000000,60.000000" (+ (Transformation|GetActorLocation) (Math|Vector|MakeVector (Math|Random|RandomFloatinRange -2e+01 2e+01) (Math|Random|RandomFloatinRange -2e+01 2e+01) -1e+02)) "-90.000000,0.000000,0.000000" 2e+01))))
    (:then_1
      (bind _asmaterial_instance_dynamic (Utilities|Casting|CastToMaterialInstanceDynamic _returnvalue_2)
        (:then
          (Rendering|Material|SetScalarParameterValue _asmaterial_instance_dynamic "Blood" _returnvalue :!class /Script/Engine.MaterialInstanceDynamic))
        (:CastFailed
          (bind _returnvalue_3 (Rendering|Material|CreateDynamicMaterialInstance _mesh 0 _returnvalue_2 "BloodDynamic" :!class /Script/Engine.PrimitiveComponent))
          (Rendering|Material|SetScalarParameterValue _returnvalue_3 "Blood" _returnvalue :!class /Script/Engine.MaterialInstanceDynamic)
          (Rendering|Material|SetMaterial _mesh 0 _returnvalue_3))))))

(event OnSwitchWeapon(InventoryComponent)
  (params (WeaponIdName :type Name :default "None") (WeaponAdditionalInfo :type Additional%20Weapon%20Info%20Structure) (NewCurrentIndexWeapon :type Integer))
  ;[1 1 1] SwitchWeapon
  (bind _asbp_player_controller (Utilities|Casting|CastToBP_PlayerController (Game|GetPlayerController 0)))
  (Utilities|IsValid (Variables|/Game/Blueprint/Game/BP_PlayerController.BP_PlayerController_C|GetInGameWidget _asbp_player_controller)
    (:Is%20Valid
      (bind _asbpw_weapon_slots (Utilities|Casting|CastToBPW_WeaponSlots (Class|PanelWidget|GetChildat (Variables|/Game/Widget/Inventory/BPW_InventoryStatsWidget.BPW_InventoryStatsWidget_C|GetWeaponSlots (Variables|/Game/Widget/BPW_InGameWidget.BPW_InGameWidget_C|GetInventoryStatsWidget (Variables|/Game/Blueprint/Game/BP_PlayerController.BP_PlayerController_C|GetInGameWidget _asbp_player_controller))) NewCurrentIndexWeapon)))
      (Default|UpdateInfo _asbpw_weapon_slots WeaponIdName (Utilities|Struct|BreakAdditionalWeaponInfo WeaponAdditionalInfo)))))

(event Custom|StartSwitchWeapon
  (params (PickUpWeapon :type BP%20Pick%20Up%20Actor%20Weapon%20Object%20Reference))
  ;[1 1 1] SwitchWeapon
  (Variables|PickUp|SetCatchPickUpWeapon PickUpWeapon))

(event Custom|EndOverlapWithPickUpWeapon
  ;[1 1 1] Interact/Drop Actor
  (bind _asbp_player_controller (Utilities|Casting|CastToBP_PlayerController (Pawn|GetController)))
  (Widget|SetVisibility (Variables|/Game/Widget/BPW_InGameWidget.BPW_InGameWidget_C|GetPickUpWidget (Variables|/Game/Blueprint/Game/BP_PlayerController.BP_PlayerController_C|GetInGameWidget _asbp_player_controller)) "Collapsed"))

(event Custom|SetColorCapeCharacter_OnServer
  (params (TrueColorCape :type Material%20Interface%20Object%20Reference))
  (Utilities|IsValid TrueColorCape
    (:Is%20Valid
      (CallFunction|SetColorCapeCharacterMulticast TrueColorCape))))

(event Custom|SetColorCapeCharacter_Multicast
  (params (TrueColorCape :type Material%20Interface%20Object%20Reference))
  (bind _cape (Variables|Default|GetCape))
  (bind _mesh (Variables|Character|GetMesh))
  (Class|SkinnedMeshComponent|SetSkeletalMesh _cape "/Game/Blueprint/Game/Lobby/Cape/SK_GothicKnight_CapeFurBlack.SK_GothicKnight_CapeFurBlack" true)
  (Rendering|Material|SetMaterial _cape 1 TrueColorCape)
  (Variables|Default|SetTrueColorCape TrueColorCape)
  (Transformation|AttachComponentToComponent (Variables|Default|GetCape) _mesh "None" "SnapToTarget" "SnapToTarget" "SnapToTarget" true)
  (Class|SkinnedMeshComponent|SetMasterPoseComponent (Variables|Default|GetCape) _mesh true))

(event Custom|CheckPickUpActor
  (bind _interactpickupactor (Variables|Default|GetInteractPickUpActor))
  (bind _overlappingactors (Collision|GetOverlappingActors _interactpickupactor "/Game/Blueprint/InteractionEnviroment/PickUpActor/BP_PickUpActor_Weapon.BP_PickUpActor_Weapon_C" :!class /Script/Engine.PrimitiveComponent))
  (bind _output (Utilities|Array|Get(acopy) _overlappingactors))
  ;[1 1 1] Interact/Drop Actor
  (bind _asbp_player_controller (Utilities|Casting|CastToBP_PlayerController (Pawn|GetController)))
  (Utilities|IsValid (Variables|/Game/Blueprint/Game/BP_PlayerController.BP_PlayerController_C|GetInGameWidget _asbp_player_controller)
    (:Is%20Valid
      (if (> (Utilities|Array|Length _overlappingactors) 0)
        (Utilities|IsValid _output
          (:Is%20Valid
            (bind _asbp_pick_up_actor_weapon (Utilities|Casting|CastToBP_PickUpActor_Weapon _output))
            (if (not (Utilities|Name|Equal(Name) (Variables|/Game/Widget/Inventory/BPW_PickUpWidget.BPW_PickUpWidget_C|GetIdWeaponName (Variables|/Game/Widget/BPW_InGameWidget.BPW_InGameWidget_C|GetPickUpWidget (Variables|/Game/Blueprint/Game/BP_PlayerController.BP_PlayerController_C|GetInGameWidget _asbp_player_controller))) (Variables|/Game/Blueprint/InteractionEnviroment/PickUpActor/BP_PickUpActor_Weapon.BP_PickUpActor_Weapon_C|GetNameItem _asbp_pick_up_actor_weapon)))
              (Default|ChangeName (Variables|/Game/Widget/BPW_InGameWidget.BPW_InGameWidget_C|GetPickUpWidget (Variables|/Game/Blueprint/Game/BP_PlayerController.BP_PlayerController_C|GetInGameWidget _asbp_player_controller)) (Utilities|Text|ToText(Name) (Variables|/Game/Blueprint/InteractionEnviroment/PickUpActor/BP_PickUpActor_Weapon.BP_PickUpActor_Weapon_C|GetNameItem _asbp_pick_up_actor_weapon)))
              (Widget|SetVisibility (Variables|/Game/Widget/BPW_InGameWidget.BPW_InGameWidget_C|GetPickUpWidget (Variables|/Game/Blueprint/Game/BP_PlayerController.BP_PlayerController_C|GetInGameWidget _asbp_player_controller)) "Visible")))
          (:Is%20Not%20Valid
            (Widget|SetVisibility (Variables|/Game/Widget/BPW_InGameWidget.BPW_InGameWidget_C|GetPickUpWidget (Variables|/Game/Blueprint/Game/BP_PlayerController.BP_PlayerController_C|GetInGameWidget _asbp_player_controller)) "Collapsed" :!label _label)))
        (else
          (goto _label))))))

(event Custom|NoiseEvent
  (Class|AISenseHearing|ReportNoiseEvent (Transformation|GetActorLocation) 1.0 self 0.0 "None"))

(event Custom|SetColorCharacter_OnServer
  (params (TrueColor :type Material%20Interface%20Object%20Reference))
  (Utilities|IsValid TrueColor
    (:Is%20Valid
      (CallFunction|SetColorCharacterMulticast TrueColor))))

(event Custom|SetColorCharacter_Multicast
  (params (TrueColor :type Material%20Interface%20Object%20Reference))
  (Rendering|Material|SetMaterial (Variables|Character|GetMesh) 0 TrueColor)
  (Variables|Default|SetTrueColor TrueColor))

(event Custom|ReloadAnimEnd_Multicast
  (params (bIsSuccess :type Boolean))
  ;[1 1 1] Weapon Reload/Fire
  (Default|ReloadingEnd (Variables|Default|GetAnimationInstance) bIsSuccess))

(event Custom|FireAnimStart_Multicast
  (params (MontageToPlay :type Anim%20Montage%20Object%20Reference))
  ;[1 1 1] Weapon Reload/Fire
  (Default|Firing (Variables|Default|GetAnimationInstance) MontageToPlay))

(event Custom|ActivateCheckPickUpActor
  (Utilities|Time|SetTimerbyEvent (delegate Custom|CheckPickUpActor) 0.4 true))

(event Custom|ReloadAnimStart_Multicast
  (params (MontageToPlay :type Anim%20Montage%20Object%20Reference))
  ;[1 1 1] Weapon Reload/Fire
  (Default|Reloading (Variables|Default|GetAnimationInstance) MontageToPlay))

(event EventWeaponFireBP
  (params (Anim :type Anim%20Montage%20Object%20Reference))
  ;[1 1 1] Weapon Reload/Fire
  (CallFunction|FireAnimStartMulticast Anim))

(event EventBeginPlay
  (Utilities|FlowControl|Sequence
    (:then_0
      (bind _asabp_third_person (Utilities|Casting|CastToABP_ThirdPerson (Components|SkeletalMesh|GetAnimInstance (Variables|Character|GetMesh))))
      (Variables|Default|SetAnimationInstance _asabp_third_person)
      (Networking|SwitchHasAuthority
        (:Authority
          (Utilities|Time|SetTimerbyEvent (delegate Custom|NoiseEvent) 1.0 true))))
    (:then_1
      (if (Utilities|Enum|Equal(Enum) (Networking|GetLocalRole) "ROLE_SimulatedProxy")
        (Rendering|Material|SetMaterial (Variables|Character|GetMesh) 0 (Variables|Default|GetTrueColor))))
    (:then_2
      (if (Utilities|Enum|Equal(Enum) (Networking|GetLocalRole) "ROLE_SimulatedProxy")
        (Class|SkinnedMeshComponent|SetSkeletalMesh (Variables|Default|GetCape) "/Game/Blueprint/Game/Lobby/Cape/SK_GothicKnight_CapeFurBlack.SK_GothicKnight_CapeFurBlack" true)
        (Transformation|AttachComponentToComponent (Variables|Default|GetCape) (Variables|Character|GetMesh) "None" "SnapToTarget" "SnapToTarget" "SnapToTarget" true)
        (Class|SkinnedMeshComponent|SetMasterPoseComponent (Variables|Default|GetCape) (Variables|Character|GetMesh) true)
        (Rendering|Material|SetMaterial (Variables|Default|GetCape) 1 (Variables|Default|GetTrueColorCape))))))

(event EventDropWeapontoWorld
  (params (DropItemInfo :type Drop%20Item%20Structure))
  ;[1 1 1] Interact/Drop Actor
  (|CallParentFunction DropItemInfo)
  (CallFunction|DropItem DropItemInfo))

(event EventWeaponReloadEndBP
  (params (bIsSuccess :type Boolean))
  ;[1 1 1] Weapon Reload/Fire
  (CallFunction|ReloadAnimEndMulticast bIsSuccess)
  (bind _asbp_player_controller (Utilities|Casting|CastToBP_PlayerController (Game|GetPlayerController 0)))
  (Utilities|IsValid (Variables|/Game/Blueprint/Game/BP_PlayerController.BP_PlayerController_C|GetInGameWidget _asbp_player_controller)
    (:Is%20Valid
      (Default|WeaponReloadEnd (Variables|/Game/Widget/BPW_InGameWidget.BPW_InGameWidget_C|GetInventoryStatsWidget (Variables|/Game/Blueprint/Game/BP_PlayerController.BP_PlayerController_C|GetInGameWidget _asbp_player_controller)) (Class|TDSCharacter|GetCurrentWeaponIndex) bIsSuccess))))

(event EventWeaponReloadStartBP
  (params (Anim :type Anim%20Montage%20Object%20Reference))
  ;[1 1 1] Weapon Reload/Fire
  (CallFunction|ReloadAnimStartMulticast Anim)
  (bind _asbp_player_controller (Utilities|Casting|CastToBP_PlayerController (Game|GetPlayerController 0)))
  (Utilities|IsValid (Variables|/Game/Blueprint/Game/BP_PlayerController.BP_PlayerController_C|GetInGameWidget _asbp_player_controller)
    (:Is%20Valid
      (Default|WeaponReloadStart (Variables|/Game/Widget/BPW_InGameWidget.BPW_InGameWidget_C|GetInventoryStatsWidget (Variables|/Game/Blueprint/Game/BP_PlayerController.BP_PlayerController_C|GetInGameWidget _asbp_player_controller)) (Class|TDSCharacter|GetCurrentWeaponIndex)))))

(event EventPossessed
  (params (NewController :type Controller%20Object%20Reference))
  (CallFunction|ActivateCheckPickUpActor))

(event EventCharacterDeadBP
  ;[1 1 1] Dead
  (Networking|SwitchHasAuthority
    (:Authority
      (bind _asbp_player_controller (Utilities|Casting|CastToBP_PlayerController (Pawn|GetController)))
      (bind _output_get (Variables|Default|SetController_T _asbp_player_controller))
      (Pawn|UnPossess _output_get)
      (bind _asbp_game_mode (Utilities|Casting|CastToBP_GameMode (Game|GetGameMode)))
      (bind _bsuccess (Default|TrytoRespawnPlayer _asbp_game_mode (Variables|Default|GetController_T)))
      (if (not _bsuccess)
        (Default|TrytoRespawnPlayeratSpectactor _asbp_game_mode (Variables|Default|GetController_T))
        (Components|DestroyComponent (Variables|Default|GetCape))))))

(event EventUnpossessed
  (params (OldController :type Controller%20Object%20Reference))
  (bind _inventorycomponent (Variables|Default|GetInventoryComponent))
  ;[1 1 1] Dead
  (bind _asbp_player_state (Utilities|Casting|CastToBP_PlayerState (Variables|/Script/Engine.Controller|GetPlayerState OldController)))
  (bind _returnvalue (Class|TDSInventoryComponent|GetWeaponSlots _inventorycomponent))
  (bind _returnvalue_2 (Class|TDSInventoryComponent|GetAmmoSlots _inventorycomponent))
  (Default|SaveCurrentInventory _asbp_player_state _returnvalue _returnvalue_2))

(event Input|ActionEvents|InputActionInteractPickUpActor
  (params (Key :type Key%20Structure :default "None"))
  ;[1 1 1] Interact/Drop Actor
  (:Pressed
    (Variables|PickUp|SetInteractKeyPressed true)
    (bind _returnvalue (Utilities|Time|SetTimerbyFunctionName 0 "TryPickUpActorPressed" (Variables|PickUp|GetPickUpTime)))
    (bind _output_get (Variables|PickUp|SetPickUpPressedTimer _returnvalue))
    (bind _asbp_player_controller (Utilities|Casting|CastToBP_PlayerController (Pawn|GetController)))
    (Utilities|IsValid (Variables|/Game/Widget/BPW_InGameWidget.BPW_InGameWidget_C|GetPickUpWidget (Variables|/Game/Blueprint/Game/BP_PlayerController.BP_PlayerController_C|GetInGameWidget _asbp_player_controller))
      (:Is%20Valid
        (Variables|/Game/Widget/Inventory/BPW_PickUpWidget.BPW_PickUpWidget_C|SetTimer (Variables|/Game/Widget/BPW_InGameWidget.BPW_InGameWidget_C|GetPickUpWidget (Variables|/Game/Blueprint/Game/BP_PlayerController.BP_PlayerController_C|GetInGameWidget _asbp_player_controller)) _output_get))))
  (:Released
    (Variables|PickUp|SetInteractKeyPressed false)
    (Utilities|Time|ClearandInvalidateTimerbyHandle (Variables|PickUp|GetPickUpPressedTimer))))

(fn ConstructionScript
  (bind _cameraboom (Variables|Default|GetCameraBoom))
  (Variables|/Script/Engine.SpringArmComponent|SetTargetArmLength _cameraboom (Variables|Camera|GetHeightCameraMax))
  (Transformation|SetRelativeRotation _cameraboom (Variables|Camera|GetRotaterCamera) false false)
  (Variables|/Script/Engine.SpringArmComponent|SetbEnableCameraLag _cameraboom (Variables|Camera|GetFlow))
  (Variables|/Script/Engine.SpringArmComponent|SetCameraLagSpeed _cameraboom (Variables|Camera|GetCoefSmooth)))

(fn CameraSlide
  (params (A :type Float%20%28single-precision%29) (A2 :type Float%20%28single-precision%29))
  (bind _returnvalue (* 50 1.0))
  (bind _cameraboom (Variables|Default|GetCameraBoom))
  (if (!= A2 0.0)
    (if (> A 0.0)
      (if (> (- (Variables|/Script/Engine.SpringArmComponent|GetTargetArmLength _cameraboom) _returnvalue) (Variables|Camera|GetHeightCameraMin))
        (Variables|Camera|SetSlideUp true)
        (Variables|/Script/Engine.SpringArmComponent|SetTargetArmLength _cameraboom (- (Variables|/Script/Engine.SpringArmComponent|GetTargetArmLength _cameraboom) _returnvalue))
        (bind _returnvalue_2 (Utilities|Time|SetTimerbyFunctionName 0 "CameraSlideSmoothTick" 0.001 true :!label _label))
        (Variables|Camera|SetSlideTimer _returnvalue_2))
      (elif (< (+ (Variables|/Script/Engine.SpringArmComponent|GetTargetArmLength _cameraboom) _returnvalue) (Variables|Camera|GetHeightCameraMax))
        (Variables|Camera|SetSlideUp false)
        (Variables|/Script/Engine.SpringArmComponent|SetTargetArmLength _cameraboom (+ (Variables|/Script/Engine.SpringArmComponent|GetTargetArmLength _cameraboom) _returnvalue))
        (goto _label)))))

(fn CameraSlideSmoothTick
  (bind _camerachangeslidestepdistance (Variables|Camera|GetCameraChangeSlideStepDistance))
  (bind _cameraboom (Variables|Default|GetCameraBoom))
  (bind _output_get (Variables|Camera|SetCurrentSlideDistance (+ (Variables|Camera|GetCurrentSlideDistance) _camerachangeslidestepdistance)))
  (Variables|/Script/Engine.SpringArmComponent|SetTargetArmLength _cameraboom (select (Variables|Camera|GetSlideUp) (- (Variables|/Script/Engine.SpringArmComponent|GetTargetArmLength _cameraboom) _camerachangeslidestepdistance) (+ (Variables|/Script/Engine.SpringArmComponent|GetTargetArmLength _cameraboom) _camerachangeslidestepdistance)))
  (if (>= _output_get (Variables|Camera|GetHighCameraChangeDistance))
    (Variables|Camera|SetCurrentSlideDistance 0.0)
    (Utilities|Time|ClearandInvalidateTimerbyHandle (Variables|Camera|GetSlideTimer))))

(fn DropItem
  (params (DropItemInfo :type Drop%20Item%20Structure))
  (Game|SpawnActorfromClass "/Game/Blueprint/InteractionEnviroment/PickUpActor/BP_PickUpActor_Weapon.BP_PickUpActor_Weapon_C" (Math|Transform|MakeTransform (+ (Transformation|GetActorLocation) (* (Transformation|GetActorForwardVector) 1e+02))) "AdjustIfPossibleButAlwaysSpawn" 0 DropItemInfo 0))

(fn TryPickUpActorPressed
  (bind _interactpickupactor (Variables|Default|GetInteractPickUpActor))
  (bind _overlappingactors (Collision|GetOverlappingActors _interactpickupactor "/Game/Blueprint/InteractionEnviroment/PickUpActor/BP_PickUpActor_Weapon.BP_PickUpActor_Weapon_C" :!class /Script/Engine.PrimitiveComponent))
  (bind _output (Utilities|Array|Get(acopy) _overlappingactors))
  (Utilities|IsValid _output
    (:Is%20Valid
      (bind _asbp_pick_up_actor_weapon (Utilities|Casting|CastToBP_PickUpActor_Weapon _output))
      (Class|TDSInventoryComponent|TryGetWeapontoInventoryonServer (Variables|Default|GetInventoryComponent) _asbp_pick_up_actor_weapon (Utilities|Struct|BreakDropItem (Variables|/Game/Blueprint/InteractionEnviroment/PickUpActor/BP_PickUpActor_Weapon.BP_PickUpActor_Weapon_C|GetWeaponInfo _asbp_pick_up_actor_weapon))))))