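; BP_KillScoreComponent is an actor component that hands out a Score value when its owning enemy dies.
; On the server it binds to the owner's TDSHealthComponent death event at BeginPlay.
; The death handler reports Score to BP_GameMode through EnemyDead, then passes it to SetScore on the last instigator's BP_PlayerState.
; The component destroys itself after scoring, or through a separate Destroy event.
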(event Custom|DeadOwner
  (bind _asbp_game_mode (Utilities|Casting|CastToBP_GameMode (Game|GetGameMode)))
  (Default|EnemyDead _asbp_game_mode (Variables|Default|GetScore))
  (bind _asbp_character_enemy_base (Utilities|Casting|CastToBP_CharacterEnemy_Base (Components|GetOwner)))
  (bind _asbp_player_state (Utilities|Casting|CastToBP_PlayerState (Variables|/Script/Engine.Controller|GetPlayerState (Variables|/Game/Blueprint/EnemyCharacter/BP_CharacterEnemy_Base.BP_CharacterEnemy_Base_C|GetLastInstigator _asbp_character_enemy_base))))
  (Default|SetScore _asbp_player_state (Variables|Default|GetScore))
  (Components|DestroyComponent))

(event Custom|Destroy
  (Components|DestroyComponent))

(event EventBeginPlay
  (if (Networking|IsServer)
    (EventDispatchers|BindEventtoOnDead (Actor|GetComponentbyClass (Components|GetOwner) "/Script/TDS.TDSHealthComponent") (EventDispatchers|CreateEvent :!event Custom|DeadOwner))))