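; AI controller for the boss enemy that starts its behavior tree and chooses which player pawn it targets.
; One second after BeginPlay it runs BT_AI_Boss and writes the last PlayerArray entry's pawn to the TargetActor blackboard key.
; A one-shot timer five seconds later replaces that target once with the player pawn nearest the boss, found by GetCloseTarget's distance scan.
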(event Custom|InitBoss
  (bind _returnvalue (Game|GetGameState))
  (bind _playerarray (Variables|/Script/Engine.GameStateBase|GetPlayerArray _returnvalue))
  (bind _returnvalue_2 (Utilities|Array|Length _playerarray))
  (bind _returnvalue_3 (- _returnvalue_2 1))
  (bind _output (Utilities|Array|Get(acopy) _playerarray _returnvalue_3))
  (bind _pawnprivate (Variables|/Script/Engine.PlayerState|GetPawnPrivate _output))
  (AI|RunBehaviorTree "/Game/Blueprint/EnemyCharacter_Boss/AI/BT_AI_Boss.BT_AI_Boss")
  (Utilities|IsValid _pawnprivate
    (:Is%20Valid
      (AI|Components|Blackboard|SetValueasObject (AI|GetBlackboard 0) (Utilities|Name|MakeLiteralName "TargetActor") _pawnprivate))
    (:Is%20Not%20Valid
      _))
  (Utilities|Time|SetTimerbyEvent (delegate Custom|ReInitTarget) 5.0))

(event Custom|ReInitTarget
  (bind _closetarget (CallFunction|GetCloseTarget))
  (AI|Components|Blackboard|SetValueasObject (AI|GetBlackboard 0) (Utilities|Name|MakeLiteralName "TargetActor") _closetarget))

(event EventBeginPlay
  (Utilities|Time|SetTimerbyEvent (delegate Custom|InitBoss) 1.0))

(fn ConstructionScript)

(fn GetCloseTarget
  (bind _returnvalue (Game|GetGameState))
  (bind _playerarray (Variables|/Script/Engine.GameStateBase|GetPlayerArray _returnvalue))
  (for (_array_element _array_index) _playerarray
    (Utilities|IsValid (Variables|/Script/Engine.PlayerState|GetPawnPrivate _array_element)
      (:Is%20Valid
        (if (== _array_index 0)
          (LocalVariables|SetLenghtBetweenOwnTarget (Math|Vector|VectorLength (- (Transformation|GetActorLocation (Pawn|GetControlledPawn)) (Transformation|GetActorLocation (Variables|/Script/Engine.PlayerState|GetPawnPrivate _array_element)))))
          (LocalVariables|SetIndex 0)
          (elif (not (<= (LocalVariables|GetLenghtBetweenOwnTarget) (Math|Vector|VectorLength (- (Transformation|GetActorLocation (Pawn|GetControlledPawn)) (Transformation|GetActorLocation (Variables|/Script/Engine.PlayerState|GetPawnPrivate _array_element))))))
            (LocalVariables|SetLenghtBetweenOwnTarget (Math|Vector|VectorLength (- (Transformation|GetActorLocation (Pawn|GetControlledPawn)) (Transformation|GetActorLocation (Variables|/Script/Engine.PlayerState|GetPawnPrivate _array_element)))))
            (LocalVariables|SetIndex _array_index))))))
  (Utilities|IsValid (Utilities|Array|Get(acopy) _playerarray (LocalVariables|GetIndex))
    (:Is%20Valid
      (Utilities|IsValid (Variables|/Script/Engine.PlayerState|GetPawnPrivate (Utilities|Array|Get(acopy) _playerarray (LocalVariables|GetIndex)))
        (:Is%20Valid
          (return (Variables|/Script/Engine.PlayerState|GetPawnPrivate (Utilities|Array|Get(acopy) _playerarray (LocalVariables|GetIndex)))))
        (:Is%20Not%20Valid
          _)))
    (:Is%20Not%20Valid
      _))
  (return 0))