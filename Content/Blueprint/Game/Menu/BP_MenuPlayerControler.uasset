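; Player controller for the menu that sets up the camera view and UI for the local player.
; On BeginPlay it points the view at a CameraActor found in the level, then creates the HUD widget and adds it to the viewport.
; It pushes the menu widget onto the HUD's MenuStack and exposes that stack through a validity-checked getter.
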(event EventBeginPlay
  (bind _returnvalue (Game|GetPlayerController 0))
  (if (Pawn|IsLocalPlayerController)
    (bind _returnvalue_2 (Actor|GetActorOfClass "/Script/Engine.CameraActor"))
    (Game|Player|SetViewTargetwithBlend _returnvalue _returnvalue_2 0.0 "VTBlend_Linear" 0.0 false)
    (bind _returnvalue_3 (UserInterface|CreateWidget "/Game/Widget/Additional/WBP_HUD.WBP_HUD_C" _returnvalue))
    (Variables|Default|SetHUD _returnvalue_3)
    (UserInterface|Viewport|AddtoViewport (Variables|Default|GetHUD) 0)
    (Class|CommonActivatableWidgetContainerBase|AddWidget (Variables|/Game/Widget/Additional/WBP_HUD.WBP_HUD_C|GetMenuStack (Variables|Default|GetHUD)) "/Game/Widget/Menu/BPW_Menu.BPW_Menu_C")))

(fn ConstructionScript)

(fn GetMenuStack
  (bind _hud (Variables|Default|GetHUD)
    (:then
      (return (Variables|/Game/Widget/Additional/WBP_HUD.WBP_HUD_C|GetMenuStack _hud)))
    (:else)))