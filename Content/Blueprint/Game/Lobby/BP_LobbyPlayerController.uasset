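; Lobby player controller that links each player's lobby menu, lobby character and BP_LobbyMode.
; On local BeginPlay it shows the cursor, views through a level CameraActor and pushes BPW_LobbyMenu onto the HUD's menu stack, initialised for server or client.
; Events forward map, cape and color picks to the game mode, and others update the menu or the saved character's readiness and appearance.
; When destroyed on authority, it also destroys that character.
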(event Custom|UpdateMeReady
  (Default|MeReadyMulticast (Variables|Default|GetLobbyCharacter)))

(event Custom|UpdatePlayerSelectedMap
  (params (CurrentLevelByServer :type Name))
  (bind _asbp_lobby_mode (Utilities|Casting|CastToBP_LobbyMode (Game|GetGameMode)))
  (Default|UpdateLevelName _asbp_lobby_mode CurrentLevelByServer))

(event Custom|UpdateLobbyCharacterCapeParam
  (params (NewCape :type Skeletal%20Mesh%20Object%20Reference) (NewColorCape :type Material%20Interface%20Object%20Reference))
  (Default|ChangeCapeonServer (Variables|Default|GetLobbyCharacter) NewCape NewColorCape))

(event Custom|UpdateLobbyWidgetOnClient
  (params (Name :type Name))
  (Default|UpdateLevelName (Variables|Default|GetLobbyMenu) Name))

(event Custom|UpdatePlayerName
  (params (InText :type Text))
  (Rendering|Components|TextRender|SetText (Variables|/Game/Widget/Menu/LobbyMenu/BPW_LobbyMenu.BPW_LobbyMenu_C|GetPlayerName (Variables|Default|GetLobbyMenu)) InText))

(event Custom|SelectedNewColor
  (params (Color :type Material%20Interface%20Object%20Reference))
  (bind _asbp_lobby_mode (Utilities|Casting|CastToBP_LobbyMode (Game|GetGameMode)))
  (Default|UpdateColorforCharacter _asbp_lobby_mode Color self))

(event Custom|SaveLobbyCharacter
  (params (LobbyCharacter :type BP%20Lobby%20Character%20Object%20Reference))
  (Variables|Default|SetLobbyCharacter LobbyCharacter))

(event Custom|UpdateColorsLobbyWidget_OnClient
  (params (BlockColors :type Array%20of%20Material%20Interface%20Object%20References))
  (bind _lobbymenu (Variables|Default|GetLobbyMenu))
  (Utilities|IsValid _lobbymenu
    (:Is%20Valid
      (Default|UpdateAviableColor _lobbymenu BlockColors))))

(event Custom|UpdateLobbyCharacterColorParam
  (params (NewColor :type Material%20Interface%20Object%20Reference))
  (Default|ChangeColoronServer (Variables|Default|GetLobbyCharacter) NewColor))

(event Custom|RemoveAllWidget
  (Viewport|RemoveAllWidgets))

(event Custom|SelectedNewCape
  (params (Cape :type Skeletal%20Mesh%20Object%20Reference) (ColorCape :type Material%20Interface%20Object%20Reference))
  (bind _asbp_lobby_mode (Utilities|Casting|CastToBP_LobbyMode (Game|GetGameMode)))
  (Default|UpdateCapeforCharacter _asbp_lobby_mode self Cape ColorCape))

(event EventBeginPlay
  (if (Pawn|IsLocalPlayerController)
    (Variables|Default|SetbShowMouseCursor true)
    (bind _returnvalue (Actor|GetActorOfClass "/Script/Engine.CameraActor"))
    (Game|Player|SetViewTargetwithBlend _returnvalue 0.0 "VTBlend_Linear" 0.0 false)
    (bind _returnvalue_2 (UserInterface|CreateWidget "/Game/Widget/Additional/WBP_HUD.WBP_HUD_C"))
    (Variables|Default|SetHUD _returnvalue_2)
    (UserInterface|Viewport|AddtoViewport (Variables|Default|GetHUD) 0)
    (bind _returnvalue_3 (Class|CommonActivatableWidgetContainerBase|AddWidget (Variables|/Game/Widget/Additional/WBP_HUD.WBP_HUD_C|GetMenuStack (Variables|Default|GetHUD)) "/Game/Widget/Menu/LobbyMenu/BPW_LobbyMenu.BPW_LobbyMenu_C"))
    (bind _output_get (Variables|Default|SetLobbyMenu _returnvalue_3))
    (Default|InitServerClientWidget _output_get (Networking|IsServer))))

(event EventDestroyed
  (Networking|SwitchHasAuthority
    (:Authority
      (Actor|DestroyActor (Variables|Default|GetLobbyCharacter)))))

(fn ConstructionScript)