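; Lobby character that displays a player's chosen body color and cape, and plays a montage on ready-up.
; Server events forward cosmetic changes to multicasts that set the body material or cape mesh and store the choice.
; The cape snaps to the body's root socket and follows its animation through master pose.
; On remote BeginPlay, the stored body material and cape attachment are reapplied, but the cape mesh and stored cape color are not.
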(event Custom|ChangeColor_OnServer
  (params (TrueColor :type Material%20Interface%20Object%20Reference))
  (CallFunction|ChangeColorMulticast TrueColor))

(event Custom|ChangeColor_Multicast
  (params (NewColor :type Material%20Interface%20Object%20Reference))
  (Rendering|Material|SetMaterial (Variables|Default|GetSkeletalMesh) 0 NewColor)
  (Variables|Default|SetTrueColor NewColor))

(event Custom|MeReady_Multicast
  (Animation|Montage|PlayMontage (Variables|Default|GetSkeletalMesh) "/Game/Characters/Player/Mannequin/Animations/NewAnim/NewIdle_Rifle_Hip_Montage.NewIdle_Rifle_Hip_Montage"))

(event Custom|ChangeCape_OnServer
  (params (TrueCape :type Skeletal%20Mesh%20Object%20Reference) (TrueColorCape :type Material%20Interface%20Object%20Reference))
  (CallFunction|ChangeCapeMulticast TrueCape TrueColorCape))

(event Custom|ChangeCape_Multicast
  (params (NewCape :type Skeletal%20Mesh%20Object%20Reference) (NewColorCape :type Material%20Interface%20Object%20Reference))
  (bind _cape (Variables|Default|GetCape))
  (bind _skeletalmesh (Variables|Default|GetSkeletalMesh))
  (Class|SkinnedMeshComponent|SetSkeletalMesh (Variables|Default|GetCape) NewCape false)
  (Variables|Default|SetTrueCape NewCape)
  (Variables|Default|SetTrueColorCape NewColorCape)
  (Transformation|AttachComponentToComponent _cape _skeletalmesh "root" "SnapToTarget" "KeepRelative" "KeepWorld" true)
  (Class|SkinnedMeshComponent|SetMasterPoseComponent _cape _skeletalmesh true))

(event EventBeginPlay
  (bind _cape (Variables|Default|GetCape))
  (bind _skeletalmesh (Variables|Default|GetSkeletalMesh))
  (Networking|SwitchHasAuthority
    (:Remote
      (Rendering|Material|SetMaterial (Variables|Default|GetSkeletalMesh) 0 (Variables|Default|GetTrueColor))
      (Transformation|AttachComponentToComponent _cape _skeletalmesh "root" "SnapToTarget" "KeepRelative" "KeepWorld" true)
      (Class|SkinnedMeshComponent|SetMasterPoseComponent _cape _skeletalmesh true))))

(fn ConstructionScript)