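; Lobby player state that keeps a cached copy of the player's name and shows it in the lobby menu.
; BeginPlay stores the player name as text in CachedPlayerName, a RepNotify variable.
; Its notify casts the owner to BP_LobbyPlayerController and, if that controller's LobbyMenu is valid, writes the name into the menu's PlayerName text.
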(event EventBeginPlay
  (Variables|Default|SetCachedPlayerName (Utilities|Text|ToText(String) (PlayerState|GetPlayerName))))

(fn ConstructionScript)

(fn OnRepCachedPlayerName
  (bind _asbp_lobby_player_controller (Utilities|Casting|CastToBP_LobbyPlayerController (Components|GetOwner)))
  (Utilities|IsValid (Variables|/Game/Blueprint/Game/Lobby/BP_LobbyPlayerController.BP_LobbyPlayerController_C|GetLobbyMenu _asbp_lobby_player_controller)
    (:Is%20Valid
      (Rendering|Components|TextRender|SetText (Variables|/Game/Widget/Menu/LobbyMenu/BPW_LobbyMenu.BPW_LobbyMenu_C|GetPlayerName (Variables|/Game/Blueprint/Game/Lobby/BP_LobbyPlayerController.BP_LobbyPlayerController_C|GetLobbyMenu _asbp_lobby_player_controller)) (Variables|Default|GetCachedPlayerName)))))