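; Player controller that sets up the local UI and links the possessed BP_Character to player data.
; On possess it creates the HUD and in-game widgets, initializes inventory from BP_PlayerState slots, binds inventory and health displays, and applies body and cape colors.
; Color OnRep functions reapply colors through the character's server calls, while unpossess unbinds and removes the in-game widget.
; The menu key and game end share a toggle for the end-game widget on the HUD's pause stack.
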(event Custom|InitWidget
  (params (Weapons :type Array%20of%20Weapon%20Slot%20Structures))
  (bind _returnvalue (Pawn|GetControlledPawn))
  (Utilities|IsValid _returnvalue
    (:Is%20Valid
      (bind _asbp_character (Utilities|Casting|CastToBP_Character _returnvalue))
      (bind _ingamewidget (Variables|Default|GetInGameWidget)
        (:then
          (Default|BindInventoryEvents (Variables|/Game/Widget/BPW_InGameWidget.BPW_InGameWidget_C|GetInventoryStatsWidget _ingamewidget) _asbp_character)
          (Default|InitInventorySlots (Variables|/Game/Widget/BPW_InGameWidget.BPW_InGameWidget_C|GetInventoryStatsWidget _ingamewidget) Weapons)
          (Default|InitWidget (Variables|/Game/Widget/BPW_InGameWidget.BPW_InGameWidget_C|GetHealthBar _ingamewidget) _asbp_character))
        (:else)))))

(event Custom|UnbindWidgetEvents
  (params (Object :type Object%20Object%20Reference))
  (CallFunction|UnbindWidgets Object))

(event Custom|EndGame_PlayerController
  (params (bIsWin :type Boolean))
  (bind _endgamewidget (CallFunction|ShowEndGame))
  (Utilities|IsValid _endgamewidget
    (:Is%20Valid
      (Default|InitWidgetEndGame _endgamewidget bIsWin (Networking|IsServer)))))

(event Custom|UpdatePlayerColorPawn
  (bind _asbp_character (Utilities|Casting|CastToBP_Character (Pawn|GetControlledPawn)))
  (Default|SetColorCharacteronServer _asbp_character (Variables|Default|GetPlayerColor)))

(event Custom|AddWidgets
  (bind _returnvalue (UserInterface|CreateWidget "/Game/Widget/Additional/WBP_HUD.WBP_HUD_C" self))
  (bind _output_get (Variables|Default|SetHUD _returnvalue))
  (UserInterface|Viewport|AddtoViewport _output_get 0)
  (bind _returnvalue_2 (UserInterface|CreateWidget "/Game/Widget/BPW_InGameWidget.BPW_InGameWidget_C" self))
  (bind _output_get_2 (Variables|Default|SetInGameWidget _returnvalue_2))
  (UserInterface|Viewport|AddtoViewport _output_get_2 0))

(event Custom|UpdatePlayerColorCapePawn
  (bind _asbp_character (Utilities|Casting|CastToBP_Character (Pawn|GetControlledPawn)))
  (Default|SetColorCapeCharacteronServer _asbp_character (Variables|Default|GetPlayerColorCape)))

(event EventBeginPlay
  (if (Pawn|IsLocalPlayerController)
    (Audio|PushSoundMixModifier "/Game/Sounds/Mix_Main.Mix_Main")))

(event EventUnPossess
  (params (UnpossessedPawn :type Pawn%20Object%20Reference))
  (CallFunction|UnbindWidgetEvents UnpossessedPawn)
  (bind _ingamewidget (Variables|Default|GetInGameWidget)
    (:then
      (Widget|RemovefromParent _ingamewidget)
      (Variables|Default|SetInGameWidget 0))
    (:else)))

(event EventPossess
  (params (PossessedPawn :type Pawn%20Object%20Reference))
  (Input|SetInputModeGameOnly self)
  (Variables|Default|SetbShowMouseCursor false)
  (CallFunction|AddWidgets)
  (bind _asbp_character (Utilities|Casting|CastToBP_Character (Pawn|GetControlledPawn)))
  (Variables|Default|SetControlledCharacter _asbp_character)
  (bind _asbp_player_state (Utilities|Casting|CastToBP_PlayerState (Variables|Default|GetPlayerState)))
  (Class|TDSInventoryComponent|InitInventoryonServer (Variables|/Script/TDS.TDSCharacter|GetInventoryComponent (Variables|Default|GetControlledCharacter)) (Variables|/Game/Blueprint/Game/BP_PlayerState.BP_PlayerState_C|GetWeaponSlots _asbp_player_state) (Variables|/Game/Blueprint/Game/BP_PlayerState.BP_PlayerState_C|GetAmmoSlots _asbp_player_state))
  (CallFunction|InitWidget (Variables|/Game/Blueprint/Game/BP_PlayerState.BP_PlayerState_C|GetWeaponSlots _asbp_player_state))
  (Default|SetColorCapeCharacteronServer (Variables|Default|GetControlledCharacter) (Variables|Default|GetPlayerColorCape))
  (Default|SetColorCharacteronServer (Variables|Default|GetControlledCharacter) (Variables|Default|GetPlayerColor)))

(event Input|ActionEvents|InputActionOpenMenu
  (params (Key :type Key%20Structure :default "None"))
  (:Pressed
    (bind _endgamewidget (CallFunction|ShowEndGame))
    (Utilities|IsValid _endgamewidget
      (:Is%20Valid
        (Variables|Default|SetEndGame _endgamewidget)))))

(fn ConstructionScript)

(fn UnbindWidgets
  (params (Target :type Object%20Object%20Reference))
  (bind _ingamewidget (Variables|Default|GetInGameWidget))
  (bind _ingamewidget_2 (Variables|Default|GetInGameWidget))
  (Utilities|IsValid Target
    (:Is%20Valid
      (LocalVariables|SetmyTarget Target))
    (:Is%20Not%20Valid
      (LocalVariables|SetmyTarget (Pawn|GetControlledPawn))))
  (Utilities|IsValid _ingamewidget
    (:Is%20Valid
      (Widget|SetVisibility (Variables|/Game/Widget/BPW_InGameWidget.BPW_InGameWidget_C|GetPickUpWidget _ingamewidget) "Collapsed")
      (bind _asbp_character (Utilities|Casting|CastToBP_Character (LocalVariables|GetmyTarget)))
      (Default|UnbindAllEvents (Variables|/Game/Widget/BPW_InGameWidget.BPW_InGameWidget_C|GetInventoryStatsWidget _ingamewidget_2) _asbp_character)
      (Default|UnBindWidget (Variables|/Game/Widget/BPW_InGameWidget.BPW_InGameWidget_C|GetHealthBar _ingamewidget_2)))))

(fn OnRepPlayerColor
  (CallFunction|UpdatePlayerColorPawn))

(fn OnRepPlayerColorCape
  (CallFunction|UpdatePlayerColorCapePawn))

(fn ShowEndGame
  (bind _hud (Variables|Default|GetHUD))
  (bind _pausestack (Variables|/Game/Widget/Additional/WBP_HUD.WBP_HUD_C|GetPauseStack _hud))
  (bind _returnvalue (Class|CommonActivatableWidgetContainerBase|GetActiveWidget _pausestack))
  (Utilities|IsValid _returnvalue
    (:Is%20Valid
      (Class|CommonActivatableWidgetContainerBase|RemoveWidget _pausestack _returnvalue))
    (:Is%20Not%20Valid
      (bind _returnvalue_2 (Class|CommonActivatableWidgetContainerBase|AddWidget _pausestack "/Game/Widget/BPW_EndGame.BPW_EndGame_C"))))
  (return _returnvalue_2))

(fn Debug
  (params (TextColor :type Linear%20Color%20Structure) (A :type String) (B :type String))
  (Development|PrintString (Utilities|String|Append (Utilities|String|SelectString "SERVER" "CLIENT" (Ability|HasAuthority)) " LOCAL=" (Utilities|String|ToString(Boolean) (Pawn|IsLocalPlayerController))) true true TextColor 1e+01)
  (Development|PrintString (Utilities|String|Append A B) true true TextColor 1e+01))