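; BP_DamageActorTest is a destructible test actor that takes damage, shows damage numbers and explodes on death.
; AnyDamage feeds negated damage into the TDSHealth component's server health change, whose change event spawns a BP_DispalyDamageActor at a randomly jittered offset with current health and damage.
; On death, a brief delay lets kill-score logic run first, then explosion sound and particles play and the actor is destroyed.
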(event OnHealthChange(TDSHealth)
  (params (Health :type Float%20%28single-precision%29) (Damage :type Float%20%28single-precision%29))
  (bind _returnvalue (Game|SpawnActorfromClass "/Game/Widget/Damage/BP_DispalyDamageActor.BP_DispalyDamageActor_C" (Math|Transform|MakeTransform (+ (+ (Math|Vector|MakeVector (Math|Random|RandomFloatinRange 1e+01 1e+01) (Math|Random|RandomFloatinRange -1e+01 1e+01) 0.0) (Variables|Default|GetLocalPointSpawnHealthNumber)) (Transformation|GetActorLocation))) "Undefined" 0 0))
  (Default|InitActor _returnvalue Health Damage))

(event OnDead(TDSHealth)
  (Utilities|FlowControl|Delay 0.01) ; Before destroy must run KillScoreComp (bind TDS Health)
  (CallFunction|DestroyActor))

(event EventTick
  (params (DeltaSeconds :type Float%20%28single-precision%29)))

(event Game|Damage|EventAnyDamage
  (params (Damage :type Float%20%28single-precision%29) (DamageType :type Damage%20Type%20Object%20Reference) (InstigatedBy :type Controller%20Object%20Reference) (DamageCauser :type Actor%20Object%20Reference))
  (Class|TDSHealthComponent|ChangeHealthValueonServer (Variables|Default|GetTDSHealth) (* Damage -1.0)))

(fn ConstructionScript)

(fn DestroyActor
  (bind _returnvalue (Transformation|GetActorLocation))
  (Audio|SpawnSoundatLocation "/Game/FX_Effect/Sound/Explosion02.Explosion02" _returnvalue "0, 0, 0" 1.0 1.0 0.0 0 0)
  (Effects|SpawnEmitteratLocation "/Game/FX_Effect/Particles/P_Explosion.P_Explosion" _returnvalue)
  (Actor|DestroyActor))