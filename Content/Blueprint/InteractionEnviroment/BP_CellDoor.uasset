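; BP_CellDoor is a cell door that swings open once when a Character enters its trigger box.
; EnterBox overlap calls Opening, which sets IsOpen and plays the OpenDoor timeline to drive SMCellDoor's relative yaw.
; The first overlap also spawns the cell sound attached to the box, guarded by IsPlaySound, then destroys that audio component immediately.
; Nothing in the graph closes the door again.
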(event OnComponentBeginOverlap(EnterBox)
  (params (OverlappedComponent :type Primitive%20Component%20Object%20Reference) (OtherActor :type Actor%20Object%20Reference) (OtherComp :type Primitive%20Component%20Object%20Reference) (OtherBodyIndex :type Integer) (bFromSweep :type Boolean) (SweepResult :type Hit%20Result%20Structure%20%28by%20ref%29))
  (Utilities|Casting|CastToCharacter OtherActor)
  (CallFunction|Opening)
  (if (not (Variables|Default|GetbIsPlaySound))
    (Variables|Default|SetbIsPlaySound true)
    (bind _returnvalue (Audio|SpawnSoundAttached "/Game/FX_Effect/Sound/CellSound_Cue.CellSound_Cue" OverlappedComponent "None" "0, 0, 0" "0, 0, 0" "KeepRelativeOffset" false 1.0 1.0 0.0 0 0))
    (Components|DestroyComponent _returnvalue)))

(event Custom|Opening
  (if (not (Variables|Default|GetbIsOpen))
    (Variables|Default|SetbIsOpen true)
    (bind _zdirection (Timeline|OpenDoor PlayFromStart)
      (:Update
        (Transformation|SetRelativeRotation (Variables|Default|GetSM_Cell_Door) (Math|Rotator|MakeRotator 0.0 0.0 _zdirection) false false)))))

(event EventBeginPlay)

(event Collision|EventActorBeginOverlap
  (params (OtherActor :type Actor%20Object%20Reference)))

(event EventTick
  (params (DeltaSeconds :type Float%20%28single-precision%29)))

(fn ConstructionScript)