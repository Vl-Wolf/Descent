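; BP_DoorSystem is a double door that opens and closes when Characters overlap its trigger boxes.
; EnterBox overlap plays the OpenCloseDoor timeline, yawing DoorRight and DoorLeft in opposite directions, and ExitBox overlap reverses it from the end.
; ISDoorOpen blocks repeated triggers, while IsPlaySound alternates the open and close sounds.
; Each attached sound component is destroyed immediately after spawning, which likely cuts the sound off.
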(event OnComponentBeginOverlap(EnterBox)
  (params (OverlappedComponent :type Primitive%20Component%20Object%20Reference) (OtherActor :type Actor%20Object%20Reference) (OtherComp :type Primitive%20Component%20Object%20Reference) (OtherBodyIndex :type Integer) (bFromSweep :type Boolean) (SweepResult :type Hit%20Result%20Structure%20%28by%20ref%29))
  (Utilities|Casting|CastToCharacter OtherActor)
  (CallFunction|Opening)
  (if (not (Variables|Default|GetbIsPlaySound))
    (Variables|Default|SetbIsPlaySound true)
    (bind _returnvalue (Audio|SpawnSoundAttached "/Game/FX_Effect/Sound/SoundOpenDoor.SoundOpenDoor" OverlappedComponent "None" "0, 0, 0" "0, 0, 0" "KeepRelativeOffset" false 1.0 1.0 0.0 0 0))
    (Components|DestroyComponent _returnvalue)))

(event OnComponentBeginOverlap(ExitBox)
  (params (OverlappedComponent :type Primitive%20Component%20Object%20Reference) (OtherActor :type Actor%20Object%20Reference) (OtherComp :type Primitive%20Component%20Object%20Reference) (OtherBodyIndex :type Integer) (bFromSweep :type Boolean) (SweepResult :type Hit%20Result%20Structure%20%28by%20ref%29))
  (Utilities|Casting|CastToCharacter OtherActor)
  (CallFunction|Closing)
  (if (Variables|Default|GetbIsPlaySound)
    (Variables|Default|SetbIsPlaySound false)
    (bind _returnvalue (Audio|SpawnSoundAttached "/Game/FX_Effect/Sound/SoundCloseDoor.SoundCloseDoor" OverlappedComponent "None" "0, 0, 0" "0, 0, 0" "KeepRelativeOffset" false 1.0 1.0 0.0 0 0))
    (Components|DestroyComponent _returnvalue)))

(event Custom|Opening
  (if (not (Variables|Default|GetbISDoorOpen))
    (Variables|Default|SetbISDoorOpen true)
    (bind _zdirection (Timeline|OpenCloseDoor PlayFromStart)
      (:Update
        (Transformation|SetRelativeRotation (Variables|Default|GetDoorRight) (Math|Rotator|MakeRotator 0.0 0.0 _zdirection) false false)
        (Transformation|SetRelativeRotation (Variables|Default|GetDoorLeft) (Math|Rotator|MakeRotator 0.0 0.0 (* -1 _zdirection)) false false)))))

(event Custom|Closing
  (if (Variables|Default|GetbISDoorOpen)
    (Variables|Default|SetbISDoorOpen false)
    (bind _zdirection (Timeline|OpenCloseDoor ReverseFromEnd)
      (:Update
        (Transformation|SetRelativeRotation (Variables|Default|GetDoorRight) (Math|Rotator|MakeRotator 0.0 0.0 _zdirection) false false)
        (Transformation|SetRelativeRotation (Variables|Default|GetDoorLeft) (Math|Rotator|MakeRotator 0.0 0.0 (* -1 _zdirection)) false false)))))

(event EventBeginPlay)

(event Collision|EventActorBeginOverlap
  (params (OtherActor :type Actor%20Object%20Reference)))

(event EventTick
  (params (DeltaSeconds :type Float%20%28single-precision%29)))

(fn ConstructionScript)