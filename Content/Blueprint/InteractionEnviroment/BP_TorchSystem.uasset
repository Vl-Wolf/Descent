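; BP_TorchSystem is an environment actor with a pair of torches that light up when a Character enters its trigger box.
; EnterBox overlap calls the Burning event, which is guarded by IsBurning so it ignites only once, with no logic to extinguish.
; Ignition applies configurable color and intensity to both FireLight components, makes them visible, and attaches a scaled Fire particle emitter to each.
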(event OnComponentBeginOverlap(EnterBox)
  (params (OverlappedComponent :type Primitive%20Component%20Object%20Reference) (OtherActor :type Actor%20Object%20Reference) (OtherComp :type Primitive%20Component%20Object%20Reference) (OtherBodyIndex :type Integer) (bFromSweep :type Boolean) (SweepResult :type Hit%20Result%20Structure%20%28by%20ref%29))
  (Utilities|Casting|CastToCharacter OtherActor)
  (CallFunction|Burning))

(event Custom|Burning
  (bind _firelight1 (Variables|Default|GetFireLight1))
  (bind _firelight2 (Variables|Default|GetFireLight2))
  (bind _firescale (Variables|Default|GetFireScale))
  (bind _fire (Variables|Default|GetFire))
  (if (not (Variables|Default|GetbIsBurning))
    (bind _output_get (Variables|Default|SetbIsBurning true))
    (Rendering|Components|Light|SetLightColor _firelight1 (Math|Conversions|ToLinearColor(Color) (Variables|Default|GetFireColor)) true)
    (Rendering|Components|Light|SetIntensity _firelight1 (Variables|Default|GetLightIntensity))
    (Rendering|SetVisibility _firelight2 _output_get false)
    (Effects|SpawnEmitterAttached _fire _firelight1 "None" "0, 0, 0" "0, 0, 0" _firescale)
    (Effects|SpawnEmitterAttached _fire _firelight2 "None" "0, 0, 0" "0, 0, 0" _firescale)))

(event EventBeginPlay)

(event Collision|EventActorBeginOverlap
  (params (OtherActor :type Actor%20Object%20Reference)))

(event EventTick
  (params (DeltaSeconds :type Float%20%28single-precision%29)))

(fn ConstructionScript)