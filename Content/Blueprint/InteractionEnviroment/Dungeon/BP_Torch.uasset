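; BP_Torch is a dungeon environment torch actor with a point light and an attached sound.
; The construction script applies exposed variables for attenuation, source radii, intensity and mobility to TorchPointLight, so each placed instance can be configured separately.
; On BeginPlay it spawns the sound attached to that light.
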(event EventBeginPlay
  (Audio|SpawnSoundAttached (Variables|Default|GetSound) (Variables|Default|GetTorch_PointLight) "None" "0, 0, 0" "0, 0, 0" "KeepRelativeOffset" false 1.0 1.0 0.0 0 0))

(fn ConstructionScript
  (bind _torch_pointlight (Variables|Default|GetTorch_PointLight))
  (Rendering|Lighting|SetAttenuationRadius _torch_pointlight (Variables|Default|GetAttenuationRadius))
  (Class|PointLightComponent|SetSoftSourceRadius _torch_pointlight (Variables|Default|GetSoftSourceRadius))
  (Class|PointLightComponent|SetSourceRadius _torch_pointlight (Variables|Default|GetSourceRadius))
  (Rendering|Components|Light|SetIntensity _torch_pointlight (Variables|Default|GetIntencity))
  (Transformation|SetMobility (Variables|Default|GetTorch_PointLight) (Variables|Default|GetLightMobility)))