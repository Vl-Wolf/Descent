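; BP_CellDoor is a dungeon cell door that swings open once, either on character overlap or when a game phase is reached.
; Normal doors open through the EnterBox overlap; phase doors disable that box and poll BP_GameState's CurrentPhase on a looping timer.
; Opening uses a one-shot flag, drives the mesh yaw with the OpenDoor timeline, and spawns a door sound whose component is immediately destroyed.
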(event OnComponentBeginOverlap(EnterBox)
  (params (OverlappedComponent :type Primitive%20Component%20Object%20Reference) (OtherActor :type Actor%20Object%20Reference) (OtherComp :type Primitive%20Component%20Object%20Reference) (OtherBodyIndex :type Integer) (bFromSweep :type Boolean) (SweepResult :type Hit%20Result%20Structure%20%28by%20ref%29))
  (Utilities|Casting|CastToCharacter OtherActor)
  (CallFunction|Opening true))

(event Custom|CheckPhase
  (bind _open (CallFunction|OpenPhaseDoor))
  (CallFunction|Opening _open))

(event Custom|Opening
  (params (Open :type Boolean))
  (if Open
    (if (not (Variables|Default|GetbIsPlaySound))
      (Variables|Default|SetbIsPlaySound true)
      (bind _returnvalue (Audio|SpawnSoundAttached "/Game/FX_Effect/Sound/CellSound_Cue.CellSound_Cue" (Variables|Default|GetEnterBox) "None" "0, 0, 0" "0, 0, 0" "KeepRelativeOffset" false 1.0 1.0 0.0 0 0))
      (Components|DestroyComponent _returnvalue)
      (bind _zdirection (Timeline|OpenDoor PlayFromStart)
        (:Update
          (Transformation|SetRelativeRotation (Variables|Default|GetSM_Cell_Door) (Math|Rotator|MakeRotator 0.0 0.0 _zdirection) false false))))))

(event EventBeginPlay
  (if (Variables|Default|GetbIsPhaseDoor)
    (Collision|SetCollisionEnabled (Variables|Default|GetEnterBox) "NoCollision")
    (Utilities|Time|SetTimerbyEvent (delegate Custom|CheckPhase) 5.0 true)))

(fn ConstructionScript)

(fn OpenPhaseDoor
  (bind _asbp_game_state (Utilities|Casting|CastToBP_GameState (Game|GetGameState)))
  (if (== (Variables|Default|GetPhase) (Variables|/Game/Blueprint/Game/BP_GameState.BP_GameState_C|GetCurrentPhase _asbp_game_state))
    (if (not (Variables|Default|GetbIsOpen))
      (bind _output_get (Variables|Default|SetbIsOpen true))
      (return _output_get))))