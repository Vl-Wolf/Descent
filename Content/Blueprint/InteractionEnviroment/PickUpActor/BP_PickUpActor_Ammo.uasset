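; Ammo pickup actor that gives the character ammo for one weapon type.
; On BeginPlay, InitActor sets the static mesh, scale and glow material from WeaponTypeAmmo, destroying the mesh component if the selected asset is invalid.
; On character overlap, it asks the inventory whether that ammo type can be taken, then adds Count to the ammo slot and calls PickUpSucces from its parent pickup logic.
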(event EventBeginPlay
  (|CallParentFunction)
  (CallFunction|InitActor))

(event Collision|EventActorBeginOverlap
  (params (OtherActor :type Actor%20Object%20Reference))
  (|CallParentFunction OtherActor) ; This node is disabled and will not be called.\nDrag off pins to build functionality.
)

(event EventTick
  (params (DeltaSeconds :type Float%20%28single-precision%29))
  (|CallParentFunction DeltaSeconds) ; This node is disabled and will not be called.\nDrag off pins to build functionality.
)

(event EventOverlapCharacter
  (params (ToInv :type TDS%20Inventory%20Component%20Object%20Reference))
  (bind _weapontypeammo (Variables|Default|GetWeaponTypeAmmo))
  (|CallParentFunction ToInv)
  (bind _returnvalue (Class|TDSInventoryComponent|CheckCanTakeAmmo ToInv _weapontypeammo))
  (if _returnvalue
    (Class|TDSInventoryComponent|AmmoSlotChangeValue ToInv _weapontypeammo (Variables|Default|GetCount))
    (CallFunction|PickUpSucces)))

(fn ConstructionScript
  (|CallParentFunction))

(fn InitActor
  (bind _staticmesh (Variables|Default|GetStaticMesh))
  (bind _weapontypeammo (Variables|Default|GetWeaponTypeAmmo))
  (bind _staticmesh_2 (Variables|Default|GetStaticMesh))
  (bind _returnvalue (Utilities|Select :Index _weapontypeammo :RifleType "/Game/FX_Effect/Material/Ammo/M_Glow_RifleAmmo.M_Glow_RifleAmmo" :ShotGunType "/Game/FX_Effect/Material/Ammo/M_Glow_ShotgunAmmo.M_Glow_ShotgunAmmo" :SniperRifle "/Game/FX_Effect/Material/Ammo/M_Glow_SniperAmmo.M_Glow_SniperAmmo" :GrenadeLauncher "/Game/FX_Effect/Material/Ammo/M_Glow_GrenadeAmmo.M_Glow_GrenadeAmmo"))
  (bind _returnvalue_2 (Utilities|Select :Index _weapontypeammo :RifleType "/Game/Items/GameActor/Weapons/Rifle/AssaultRifle_Pickup.AssaultRifle_Pickup" :ShotGunType "/Game/Items/GameActor/Weapons/Shotgun/Shotgun_Pickup.Shotgun_Pickup" :SniperRifle "/Game/Items/GameActor/Weapons/SniperRifle/SniperRifle_Pickup.SniperRifle_Pickup" :GrenadeLauncher "/Game/Items/GameActor/Weapons/GrenadeLauncher/GrenadeLauncher_Pickup.GrenadeLauncher_Pickup"))
  (Utilities|FlowControl|Sequence
    (:then_0
      (Utilities|IsValid _returnvalue_2
        (:Is%20Valid
          (Components|StaticMesh|SetStaticMesh _staticmesh_2 _returnvalue_2)
          (Transformation|SetRelativeScale3D _staticmesh_2 "4.000000,4.000000,4.000000"))
        (:Is%20Not%20Valid
          (Components|DestroyComponent _staticmesh_2))))
    (:then_1
      (Utilities|IsValid _returnvalue
        (:Is%20Valid
          (Rendering|Material|SetMaterial _staticmesh 0 _returnvalue))
        (:Is%20Not%20Valid
          (Components|DestroyComponent _staticmesh))))))