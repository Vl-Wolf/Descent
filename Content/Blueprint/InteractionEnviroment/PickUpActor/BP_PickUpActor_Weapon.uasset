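; Weapon pickup actor that represents a dropped or placed weapon in the world.
; On BeginPlay it looks up drop item info by NameItem in BP_GameInstance, otherwise using its existing WeaponInfo, and passes it to InitActor.
; InitActor keeps either the static or skeletal mesh component, destroying the other, and applies any material override to the skeletal mesh only.
; Leaving the sphere trigger notifies BP_Character that the pickup overlap has ended.
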(event OnComponentEndOverlap(Sphere)
  (params (OverlappedComponent :type Primitive%20Component%20Object%20Reference) (OtherActor :type Actor%20Object%20Reference) (OtherComp :type Primitive%20Component%20Object%20Reference) (OtherBodyIndex :type Integer))
  (bind _asbp_character (Utilities|Casting|CastToBP_Character OtherActor))
  (Default|EndOverlapwithPickUpWeapon _asbp_character))

(event EventBeginPlay
  (bind _nameitem (Variables|Default|GetNameItem))
  (|CallParentFunction)
  (if (Utilities|Name|NotEqual(Name) _nameitem "None")
    (bind _asbp_game_instance (Utilities|Casting|CastToBP_GameInstance (Game|GetGameInstance)))
    (bind (_outinfo _returnvalue) (Class|TDSGameInstance|GetDropItemInfobyName _asbp_game_instance _nameitem))
    (if _returnvalue
      (bind _output_get (Variables|Default|SetWeaponInfo _outinfo))))
  (CallFunction|InitActor _output_get))

(fn ConstructionScript
  (|CallParentFunction))

(fn InitActor
  (params (InfoActor :type Drop%20Item%20Structure))
  (bind (_weaponstaticmesh _weaponskeletalmesh _weaponmaterial _offset _weaponinfo) (Utilities|Struct|BreakDropItem InfoActor))
  (Utilities|FlowControl|Sequence
    (:then_0
      (Utilities|IsValid _weaponstaticmesh
        (:Is%20Valid
          (Components|DestroyComponent (Variables|Default|GetSkeletalMesh))
          (Components|StaticMesh|SetStaticMesh (Variables|Default|GetStaticMesh) _weaponstaticmesh))
        (:Is%20Not%20Valid
          (Utilities|IsValid _weaponskeletalmesh
            (:Is%20Valid
              (Components|DestroyComponent (Variables|Default|GetStaticMesh))
              (Class|SkinnedMeshComponent|SetSkeletalMesh (Variables|Default|GetSkeletalMesh) _weaponskeletalmesh true))
            (:Is%20Not%20Valid
              (Development|PrintString "ERROR DropItem not have any MESH"))))))
    (:then_1
      (Utilities|IsValid _weaponmaterial
        (:Is%20Valid
          (Rendering|Material|SetMaterial (Variables|Default|GetSkeletalMesh) 0 _weaponmaterial))))
    (:then_2
      (Variables|Default|SetNameItem (.NameItem (Utilities|Struct|BreakWeaponSlot _weaponinfo))))))