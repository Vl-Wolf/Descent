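; First aid pickup actor that heals the character who overlaps it.
; It extends the parent pickup's overlap event, resolving the inventory component's owner to BP_Character.
; When that character's health is below a fixed full-health threshold, it applies the pickup's Value through the HealthComponent's server health change and then marks the pickup successful.
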(event EventOverlapCharacter
  (params (ToInv :type TDS%20Inventory%20Component%20Object%20Reference))
  (|CallParentFunction ToInv)
  (bind _asbp_character (Utilities|Casting|CastToBP_Character (Components|GetOwner ToInv)))
  (bind _returnvalue (Class|TDSHealthComponent|GetCurrentHealth (Variables|/Script/TDS.TDSCharacter|GetHealthComponent _asbp_character)))
  (if (< _returnvalue 1e+02)
    (Class|TDSHealthComponent|ChangeHealthValueonServer (Variables|/Script/TDS.TDSCharacter|GetHealthComponent _asbp_character) (Variables|Default|GetValue))
    (CallFunction|PickUpSucces)))

(fn ConstructionScript
  (|CallParentFunction))